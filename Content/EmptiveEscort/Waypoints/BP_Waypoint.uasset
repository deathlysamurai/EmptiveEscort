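; BP_Waypoint is a waypoint actor that completes when an escort (BP_EscortBase) overlaps it while it is active.
; Initialize stores a Radio reference and shows the waypoint as active without announcing it.
; SetActive swaps the cylinder material and toggles the flipbook marker, updating the Active flag and pinging the Radio only when announcing.
; Completion deactivates the waypoint with an announcement and plays a 2D chime.
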(event `self.ReceiveBeginPlay`)

(event `self.ReceiveActorBeginOverlap`
  (params (OtherActor :type "Actor Object Reference"))
  (bind _continue (`self.OverlapCheck` OtherActor))
  (if _continue
    (`self.Complete`)))

(fn `Complete`
  (`self.SetActive` false true)
  (`GameplayStatics.PlaySound2D` "/Game/EmptiveEscort/Audio/A_Chime_Mono_01.A_Chime_Mono_01" 1.0 1.0 0.0 null null))

(fn `Initialize`
  (params (Radio :type "/Game/EmptiveEscort/Waypoints/BP_WaypointRadio Object Reference"))
  (set `self.Radio` Radio)
  (`self.SetActive` true))

(fn `OverlapCheck`
  (params (Actor :type "Actor Object Reference"))
  (returns (Continue :type Boolean))
  (if (`self.Active`)
    (cast `/Game/EmptiveEscort/Escort/BP_EscortBase` Actor
      (:`then`
        (return true))
      (:`CastFailed`
        _)))
  (return false))

(fn `SetActive`
  (params (Active :type Boolean) (Announce :type Boolean))
  (bind _cylinder (`self.Cylinder`))
  (if Active
    (`PrimitiveComponent.SetMaterial` _cylinder 0 (`self.ActiveMaterial`))
    (else
      (`PrimitiveComponent.SetMaterial` _cylinder 0 (`self.DisabledMaterial`))))
  (`SceneComponent.SetVisibility` (`self.PaperFlipbook`) Active false)
  (if Announce
    (bind _output_get (set `self.Active` Active))
    (message `/Game/EmptiveEscort/Waypoints/BPI_WaypointReceiver.Ping Waypoint Status` (`self.Radio`) self _output_get)))

(fn `UserConstructionScript`)