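; BP_WaypointZone is an indexed waypoint zone actor for the EmptiveEscort mode.
; Its construction script writes the Index into the Name text.
; TogglePOI adds and stores a point of interest component or destroys the stored one, and SetRadio stores a Radio value.
; The begin and end overlap events are empty, so the zone does not react to overlaps itself.
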(event `self.ReceiveActorBeginOverlap`
  (params (OtherActor :type "Actor Object Reference")))

(event `self.ReceiveActorEndOverlap`
  (params (OtherActor :type "Actor Object Reference")))

(fn `Set Radio`
  (params (Radio :type "/Game/EmptiveEscort/Waypoints/BP_WaypointRadio Object Reference"))
  (set `self.Radio` Radio))

(fn `Toggle POI`
  (params (`Add POI` :type Boolean :default true))
  (if `Add POI`
    (bind _returnvalue (`AddComponent|NODE_AddBP_PointOfInterestComponent-0`))
    (set `self.POI` _returnvalue)
    (else
      (bind _poi (`self.POI`)
        (:`then`
          (`ActorComponent.K2_DestroyComponent` _poi))
        (:`else`)))))

(fn `UserConstructionScript`
  (`TextRenderComponent.K2_SetText` (`self.Name`) (`KismetTextLibrary.Conv_StringToText` (`KismetStringLibrary.Conv_IntToString` (`self.Index`)))))