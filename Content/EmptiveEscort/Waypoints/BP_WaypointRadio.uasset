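; BP_WaypointRadio is the mission manager for escort gameplay, cycling through Rest, Mission, Return and Cleanup phases.
; It spawns waypoints at random points inside indexed zones, retrying recursively toward a minimum count, and adds an invisible return waypoint once all are cleared.
; As a broadcast hub, it relays waypoint, phase and escort progress to BPI_WaypointReceiver listeners.
; It also initializes the escort, drives the mission widget and grants weapon rewards after cleanup.
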(event `Waypoints Cleared`
  (switch `/Game/EmptiveEscort/Waypoints/EPhase` (`self.Phase`)
    (:`NewEnumerator1`
      (set `self.Phase` "NewEnumerator2")
      (`self.Announce Phase`)
      (bind _returnvalue (`|SpawnActorFromClass` "/Game/EmptiveEscort/Waypoints/WaypointVarieties/BP_Waypoint_Invisible.BP_Waypoint_Invisible_C" (`KismetMathLibrary.MakeTransform` (`self.ReturnLocation`)) "Undefined" "OverrideRootScale" null null 0 0.0 null))
      (`KismetArrayLibrary.Array_Add` (`self.WaypointArray`) _returnvalue)
      (`self.Initialize Audience`)
      (`self.Update Mission Widget` 0))
    (:`NewEnumerator2`
      (set `self.Phase` "NewEnumerator3")
      (`self.Announce Phase`)
      (`self.Update Mission Widget` 0))))

(event `self.ReceiveBeginPlay`
  (`|ExecutionSequence`
    (:`then_0`
      (`self.Gather Zones`))
    (:`then_1`
      ;[1 1 1] Build Arrays
      (bind _outactors (`GameplayStatics.GetAllActorsWithInterface` "/Game/EmptiveEscort/Waypoints/BPI_WaypointReceiver.BPI_WaypointReceiver_C"))
      (bind _output_get (set `self.RadioListeners` _outactors))
      (`KismetArrayLibrary.Array_RemoveItem` _output_get self)
      (bind _outactors_2 (`GameplayStatics.GetAllActorsOfClass` "/Game/EmptiveEscort/Waypoints/BP_WaypointBase.BP_WaypointBase_C"))
      (bind _output_get_2 (set `self.WaypointArray` _outactors_2))
      ;[1 1 1] Existing Waypoint Check
      (if (> (`KismetArrayLibrary.Array_Length` _output_get_2) 0)
        (`KismetSystemLibrary.PrintString` "Waypoint in world at start, consider removing." true true (struct :`G` 0.66 :`B` 1.0 :`A` 1.0) 8.0)))
    (:`then_2`
      (`self.Initialize Audience`))))

(event `/Game/EmptiveEscort/Waypoints/BPI_WaypointReceiver.Ping Waypoint Status`
  (params (Waypoint :type "/Game/EmptiveEscort/Waypoints/BP_WaypointBase Object Reference") (Active :type Boolean))
  (bind _waypointarray (`self.WaypointArray`))
  (bind _activewaypointcount (`self.ActiveWaypointCount`))
  (bind _returnvalue (`KismetArrayLibrary.Array_Length` _waypointarray))
  (for _array_element (`self.RadioListeners`)
    (message `/Game/EmptiveEscort/Waypoints/BPI_WaypointReceiver.Ping Waypoint Status` _array_element Waypoint Active))
  (set `self.ActiveWaypointCount` 0)
  (for _array_element_2 _waypointarray
    (if (`/Game/EmptiveEscort/Waypoints/BP_WaypointBase.Active` _array_element_2)
      (`/Engine/EditorBlueprintResources/StandardMacros.IncrementInt` _activewaypointcount)))
  (if (== _activewaypointcount 0)
    (`self.Clear Waypoints`)
    (`self.Waypoints Cleared`)
    (else
      (`self.Update Mission Widget` (- _returnvalue _activewaypointcount) _returnvalue))))

(fn `Announce Escort Progress`
  (locals (EscortProgress :type "Float (double-precision)"))
  (bind _totaldistance (`self.TotalDistance`))
  (`|ExecutionSequence`
    (:`then_0`
      (set `local.EscortProgress` (/ (- _totaldistance (`KismetMathLibrary.Vector_Distance` (`self.ReferenceLocation`) (`self.K2_GetActorLocation` (`self.Escort`)))) _totaldistance)))
    (:`then_1`
      (for _array_element (`self.RadioListeners`)
        (message `/Game/EmptiveEscort/Waypoints/BPI_WaypointReceiver.Ping Escort Progress` _array_element (`self.TotalDistance`) (`local.EscortProgress`))))))

(fn `Announce Phase`
  (bind _phase (`self.Phase`))
  (for _array_element (`self.RadioListeners`)
    (if (`KismetSystemLibrary.IsValid` _array_element)
      (message `/Game/EmptiveEscort/Waypoints/BPI_WaypointReceiver.Ping Phase` _array_element _phase)
      (message `/Game/EmptiveEscort/Waypoints/BPI_WaypointReceiver.Ping Phase` _array_element _phase)
      (else
        (`self.Tune Out` _array_element))))
  (`KismetSystemLibrary.PrintString` (`KismetStringLibrary.Concat_StrStr` "Phase Change: " (`|GetEnumeratorNameAsString` _phase)) true true (struct :`R` 0.064125 :`G` 0.568522 :`B` 0.163766 :`A` 1.0)))

(fn `Clear Waypoints`
  (bind _waypointarray (`self.WaypointArray`))
  (for _array_element _waypointarray
    (`self.K2_DestroyActor` _array_element))
  (`KismetArrayLibrary.Array_Clear` _waypointarray))

(fn `Clear Zones`
  (`BlueprintMapLibrary.Map_Clear` (`self.ZoneMap`)))

(fn `Create Mission`
  (switch `/Game/EmptiveEscort/Waypoints/EPhase` (`self.Phase`)
    (:`NewEnumerator0`
      (bind (_weapon_data _weapon_rewarded) (`/Game/EmptiveEscort/Waypoints/MissionSystem/BPFL_MissionSystem.Generate Reward Weapon`))
      (bind _new_mission (`/Game/EmptiveEscort/Waypoints/MissionSystem/BPFL_MissionSystem.New Mission`))
      (`self.Next Mission` _new_mission _weapon_data _weapon_rewarded))
    (:`NewEnumerator1`
      (`KismetSystemLibrary.PrintString` "Mission In Progress" :!label _label))
    (:`NewEnumerator2`
      (goto _label))
    (:`NewEnumerator3`
      (goto _label))))

(fn `End Phase`
  (params (`Phase to End` :type "/Game/EmptiveEscort/Waypoints/EPhase Enum" :default "NewEnumerator0"))
  (bind _phase (`self.Phase`))
  (if (`|EnumEquality` `Phase to End` _phase)
    (switch `/Game/EmptiveEscort/Waypoints/EPhase` _phase
      (:`NewEnumerator0`
        (`KismetSystemLibrary.PrintString` "End Phase called at inappropriate time / No implementation" true true (struct :`G` 0.66 :`B` 1.0 :`A` 1.0) 8.0 :!label _label))
      (:`NewEnumerator1`
        (goto _label))
      (:`NewEnumerator2`
        (goto _label))
      (:`NewEnumerator3`
        (set `self.Phase` "NewEnumerator0")
        (`Widget.RemoveFromParent` (`self.MissionInfoPanel`))
        (bind _outactors (`GameplayStatics.GetAllActorsWithTag` "Enemy")) ; Emergency Cleanup, just in case there are stragglers somehow
        (for _array_element _outactors
          (`self.K2_DestroyActor` _array_element))
        (`self.Announce Phase`)
        (`self.Give Weapon Reward` true)
        (`self.Update Mission Counter`)))
    (else
      (`KismetSystemLibrary.PrintString` "End Phase called with invalid phase" true true (struct :`G` 0.66 :`B` 1.0 :`A` 1.0) 8.0))))

(fn `Gather Zones`
  (`self.Clear Zones`)
  (bind _outactors (`GameplayStatics.GetAllActorsOfClass` "/Game/EmptiveEscort/Waypoints/BP_WaypointZone.BP_WaypointZone_C"))
  (for _array_element _outactors
    (`/Game/EmptiveEscort/Waypoints/BP_WaypointZone.Set Radio` _array_element self)
    (`BlueprintMapLibrary.Map_Add` (`self.ZoneMap`) (`/Game/EmptiveEscort/Waypoints/BP_WaypointZone.Index` _array_element) _array_element)))

(fn `Get All Zones`
  (returns (AllZones :type "Map of Integer to /Game/EmptiveEscort/Waypoints/BP_WaypointZone Object Reference"))
  (return (`self.ZoneMap`)))

(fn `Get Current Mission`
  (returns (`Current Mission` :type "/Game/EmptiveEscort/Waypoints/MissionSystem/FMission Structure") (`Active Mission` :type Boolean))
  (switch `/Game/EmptiveEscort/Waypoints/EPhase` (`self.Phase`)
    (:`NewEnumerator0`
      (return (struct) false))
    (:`NewEnumerator1`
      _)
    (:`NewEnumerator2`
      _)
    (:`NewEnumerator3`
      _))
  (return (`self.CurrentMission`) true))

(fn `Get Current Phase`
  (returns (`Current Phase` :type "/Game/EmptiveEscort/Waypoints/EPhase Enum"))
  (return (`self.Phase`)))

(fn `Give Weapon Reward`
  (params (NewParam :type Boolean :default true))
  (locals (HUD :type "/Game/EmptiveEscort/UserInterface/HUD/PlayerHUD Object Reference"))
  (if NewParam
    (bind _asplayer_character (cast `/Game/EmptiveEscort/PlayerCharacter/PlayerCharacter` (`GameplayStatics.GetPlayerPawn` 0)))
    (`/Game/EmptiveEscort/PlayerCharacter/PlayerCharacter.AddAttackComponent` _asplayer_character 0 (`.AttackClass_68_AE5F9260413AB73095F984843402FFDB` (break `/Game/EmptiveEscort/PlayerCharacter/Attacks/WeaponData/WeaponDataStruct` (`self.WeaponData`))))
    (bind _asplayer_hud (cast `/Game/EmptiveEscort/UserInterface/HUD/PlayerHUD` (`PlayerController.GetHUD` (`GameplayStatics.GetPlayerController` 0))))
    (bind _output_get (set `local.HUD` _asplayer_hud))
    (`/Game/EmptiveEscort/UserInterface/HUD/PlayerHUD.Update Attack Info HUD` _output_get)
    (bind _returnvalue (`|CreateWidget` "/Game/EmptiveEscort/UserInterface/Missions/WBP_RewardCanvas.WBP_RewardCanvas_C"))
    (`/Game/EmptiveEscort/UserInterface/Missions/WBP_RewardInfo.UpdateDisplayData` (`/Game/EmptiveEscort/UserInterface/Missions/WBP_RewardCanvas.WBP_RewardInfo` _returnvalue) (`self.WeaponData`))
    (`UserWidget.AddToViewport` _returnvalue 0)))

(fn `Initialize Audience`
  (`|ExecutionSequence`
    (:`then_0`
      ;[1 1 1] Initialize Waypoints
      (for _array_element (`self.WaypointArray`)
        (`/Game/EmptiveEscort/Waypoints/BP_WaypointBase.Initialize` _array_element self)))
    (:`then_1`
      ;[1 1 1] Check if Listeners still exist
      (for _array_element_2 (`self.RadioListeners`)
        (if (not (`KismetSystemLibrary.IsValid` _array_element_2))
          (`self.Tune Out` _array_element_2))))
    (:`then_2`
      ;[1 1 1] Initialize Escort
      (for _array_element_3 (`self.RadioListeners`)
        (bind _asbp_escort_base (cast `/Game/EmptiveEscort/Escort/BP_EscortBase` _array_element_3))
        (bind _output_get (set `self.Escort` _asbp_escort_base))
        (`/Game/EmptiveEscort/Escort/BP_EscortBase.Initialize` _output_get (`self.WaypointArray`) (`self.ReturnLocation`))))))

(fn `Mark Zones`
  (params (Zones :type "Array of Integer") (`Add POI?` :type Boolean :default true))
  (for _array_element Zones
    (`/Game/EmptiveEscort/Waypoints/BP_WaypointZone.Toggle POI` (`BlueprintMapLibrary.Map_Find` (`self.ZoneMap`) _array_element) `Add POI?`)))

(fn `Next Mission`
  (params (Mission :type "/Game/EmptiveEscort/Waypoints/MissionSystem/FMission Structure") (Weapon :type "/Game/EmptiveEscort/PlayerCharacter/Attacks/WeaponData/WeaponDataStruct Structure") (WeaponRewarded :type Boolean))
  (returns (`Mission Accepted` :type Boolean))
  (switch `/Game/EmptiveEscort/Waypoints/EPhase` (`self.Phase`)
    (:`NewEnumerator0`
      (if WeaponRewarded
        (set `self.WeaponData` Weapon)
        (set `self.WeaponRewarded` true))
      (bind _output_get (set `self.CurrentMission` Mission))
      (bind (_zones _spawnmin _spawnamount _threat_value _reward_value _waypointclass) (`/Game/EmptiveEscort/Waypoints/MissionSystem/BPFL_MissionSystem.Generate Waypoint Spawn Details` _output_get))
      (`self.SpawnWaypoints` _zones _spawnmin _spawnamount _threat_value _reward_value _waypointclass)
      (`|ExecutionSequence`
        (:`then_0`
          (set `self.TotalDistance` (`KismetMathLibrary.Vector_Distance` (`self.K2_GetActorLocation` (`KismetArrayLibrary.Array_Random` (`self.WaypointArray`))) (`self.ReturnLocation`)))
          (for _array_element (`self.WaypointArray`)
            (bind _returnvalue (`self.K2_GetActorLocation` _array_element))
            (bind _returnvalue_2 (`KismetMathLibrary.Vector_Distance` _returnvalue (`self.ReturnLocation`)))
            (if (< _returnvalue_2 (`self.TotalDistance`))
              (set `self.ReferenceLocation` _returnvalue)
              (set `self.TotalDistance` _returnvalue_2))))
        (:`then_1`
          (`self.Initialize Audience`)
          (set `self.Phase` "NewEnumerator1")
          (`self.Announce Phase`)
          (`self.Announce Escort Progress`)
          (bind _returnvalue_3 (`|CreateWidget` "/Game/EmptiveEscort/UserInterface/Missions/WBP_MissionInfo.WBP_MissionInfo_C"))
          (bind _output_get_2 (set `self.MissionInfoPanel` _returnvalue_3))
          (`UserWidget.AddToViewport` _output_get_2 0)
          (`self.Update Mission Widget` 0 (`KismetArrayLibrary.Array_Length` (`self.WaypointArray`)))
          (return true))))
    (:`NewEnumerator1`
      (`KismetSystemLibrary.PrintString` "Mission Already In Progress" :!label _label)
      (return false))
    (:`NewEnumerator2`
      (goto _label))
    (:`NewEnumerator3`
      (goto _label))))

(fn `SpawnWaypoints`
  (params (Zones :type "Array of Integer") (`Spawn Min` :type Integer) (`Spawn Amount` :type Integer) (Threat :type "Float (double-precision)") (Reward :type Integer) (WaypointClass :type "/Game/EmptiveEscort/Waypoints/BP_WaypointBase Class Reference"))
  (locals (ZoneKeys :type "Array of Integer"))
  (bind _waypointarray (`self.WaypointArray`))
  (bind _spawn_min (`local.Spawn Min`))
  (bind _returnvalue (`KismetArrayLibrary.Array_Length` _waypointarray))
  (bind (_value _returnvalue_2) (`BlueprintMapLibrary.Map_Find` (`self.ZoneMap`) (`|GetArrayItem` (`local.ZoneKeys`))))
  (bind (_origin _boxextent) (`KismetSystemLibrary.GetComponentBounds` (`/Game/EmptiveEscort/Waypoints/BP_WaypointZone.Cube` _value)))
  (bind (_returnvalue_x _returnvalue_y) (`KismetMathLibrary.BreakVector` (`KismetMathLibrary.RandomPointInBoundingBox` _origin _boxextent)))
  (for _ (range `Spawn Amount`)
    (bind _output_get (set `local.ZoneKeys` Zones))
    (`KismetArrayLibrary.Array_Shuffle` _output_get)
    (if _returnvalue_2
      (bind _returnvalue_3 (`|SpawnActorFromClass` (`local.WaypointClass`) (`KismetMathLibrary.MakeTransform` (`KismetMathLibrary.MakeVector` _returnvalue_x _returnvalue_y)) "Undefined" "OverrideRootScale" null self (`local.Reward`) (`local.Threat`) null))
      (`/Engine/EditorBlueprintResources/StandardMacros.IsValid` _returnvalue_3
        (:`Is Valid`
          (`KismetArrayLibrary.Array_Add` _waypointarray _returnvalue_3)))
      (else
        (`KismetSystemLibrary.PrintString` "Error: Zone requested not in Zone Map" true true (struct :`R` 1.0 :`G` 0.078813 :`A` 1.0)))))
  (if (not (>= _returnvalue _spawn_min))
    (`self.SpawnWaypoints` (`local.Zones`) _spawn_min (- `Spawn Amount` _returnvalue) (`local.Threat`) (`local.Reward`) (`local.WaypointClass`)) ; If there aren't enough waypoints for the minimum, run again with remaining
  ))

(fn `Tune In`
  (params (Actor :type "Actor Object Reference"))
  (if (`KismetSystemLibrary.DoesImplementInterface` Actor "/Game/EmptiveEscort/Waypoints/BPI_WaypointReceiver.BPI_WaypointReceiver_C")
    (`KismetArrayLibrary.Array_AddUnique` (`self.RadioListeners`) Actor)
    (message `/Game/EmptiveEscort/Waypoints/BPI_WaypointReceiver.Ping Phase` Actor (`self.Phase`))
    (else
      (`KismetSystemLibrary.PrintString` "Can't tune in, no attached receiver." true true (struct :`R` 1.0 :`G` 0.109888 :`B` 0.484504 :`A` 1.0) 4.0))))

(fn `Tune Out`
  (params (Actor :type "Actor Object Reference"))
  (`KismetArrayLibrary.Array_RemoveItem` (`self.RadioListeners`) Actor))

(fn `Update Mission Counter`
  (bind _missionname (`/Game/EmptiveEscort/Waypoints/MissionSystem/BPFL_MissionSystem.Get Mission Details` (`self.CurrentMission`)))
  (`KismetArrayLibrary.Array_AddUnique` (`self.CompletedMissions`) _missionname)
  (`/Engine/EditorBlueprintResources/StandardMacros.IncrementInt` (`self.MissionCount`)))

(fn `Update Mission Widget`
  (params (CurrentWaypoints :type Integer) (TotalWaypoints :type Integer))
  (locals (ThreatGenerated :type "Float (double-precision)") (RewardGenerated :type Integer) (MissionName :type Text) (WaypointCount :type Text) (DetailsText :type Text))
  (bind _wbp_missioninfooverlay (`/Game/EmptiveEscort/UserInterface/Missions/WBP_MissionInfo.WBP_MissionInfoOverlay` (`self.MissionInfoPanel`)))
  (bind _returnvalue (`KismetStringLibrary.Concat_StrStr` "Threat: " (`KismetStringLibrary.Conv_DoubleToString` (`local.ThreatGenerated`)) ", Value: " (`KismetStringLibrary.Conv_IntToString` (`local.RewardGenerated`))))
  (`self.MissionInfoPanel`
    (:`then`
      (`|ExecutionSequence`
        (:`then_0`
          (bind (_missionname _missiondescription _missiontype _zones _waypointmin _waypointmax _threatmin _threatmax _threatgenerated _reward) (`/Game/EmptiveEscort/Waypoints/MissionSystem/BPFL_MissionSystem.Get Mission Details` (`self.CurrentMission`)))
          (set `local.MissionName` _missionname)
          (set `local.ThreatGenerated` _threatgenerated)
          (set `local.RewardGenerated` _reward)
          (set `local.WaypointCount` (`KismetTextLibrary.Conv_StringToText` (`KismetStringLibrary.Concat_StrStr` (`KismetStringLibrary.Conv_IntToString` (`local.CurrentWaypoints`)) " of " (`KismetStringLibrary.Conv_IntToString` (`local.TotalWaypoints`)) " completed."))))
        (:`then_1`
          (switch `/Game/EmptiveEscort/Waypoints/EPhase` (`self.Phase`)
            (:`NewEnumerator0`
              (`Widget.RemoveFromParent` (`self.MissionInfoPanel`)))
            (:`NewEnumerator1`
              (set `local.DetailsText` (`KismetTextLibrary.Conv_StringToText` _returnvalue))
              (if (`self.WeaponRewarded`)
                (set `local.DetailsText` (`KismetTextLibrary.Conv_StringToText` (`KismetStringLibrary.Concat_StrStr` _returnvalue "\nWeapon Located"))))
              (`TextBlock.SetText` (`/Game/EmptiveEscort/UserInterface/Missions/WBP_MissionInfoOverlay.MissionName` _wbp_missioninfooverlay) (`local.MissionName`) :!label _label)
              (`TextBlock.SetText` (`/Game/EmptiveEscort/UserInterface/Missions/WBP_MissionInfoOverlay.WaypointProgress` _wbp_missioninfooverlay) (`local.WaypointCount`))
              (`TextBlock.SetText` (`/Game/EmptiveEscort/UserInterface/Missions/WBP_MissionInfoOverlay.DetailsText` _wbp_missioninfooverlay) (`local.DetailsText`)))
            (:`NewEnumerator2`
              (set `local.DetailsText` "Mission Complete\nReturning to base")
              (set `local.WaypointCount` "All Waypoints Cleared!" :!label _label_2)
              (goto _label))
            (:`NewEnumerator3`
              (set `local.DetailsText` "Enemies nearby")
              (goto _label_2))))))
    (:`else`)))

(fn `UserConstructionScript`)