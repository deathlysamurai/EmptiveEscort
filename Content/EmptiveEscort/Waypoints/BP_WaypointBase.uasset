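; BP_WaypointBase is the base escort waypoint, which completes when an escort actor overlaps it while active.
; An overlap runs the empty Objective hook, waits the timer duration, then deactivates with a chime and a Radio status ping.
; SetActive swaps sprites, toggles effects and drives an optional point of interest's visibility.
; ShowInProgress, not called here, displays text and a timer flipbook rate-scaled to that duration.
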(event `self.ReceiveBeginPlay`)

(event `self.ReceiveActorBeginOverlap`
  (params (OtherActor :type "Actor Object Reference"))
  (bind _continue (`self.OverlapCheck` OtherActor))
  (if _continue
    (`self.Objective`)
    (`KismetSystemLibrary.Delay` (`self.TimerDuration`))
    (`self.Complete`)))

(fn `Complete`
  (`self.SetActive` false true)
  (`GameplayStatics.PlaySound2D` "/Game/EmptiveEscort/Audio/A_Chime_Mono_01.A_Chime_Mono_01" 1.0 1.0 0.0 null null))

(fn `Initialize`
  (params (Radio :type "/Game/EmptiveEscort/Waypoints/BP_WaypointRadio Object Reference"))
  (set `self.Radio` Radio)
  (`self.SetActive` true))

(fn `Objective`)

(fn `OverlapCheck`
  (params (Actor :type "Actor Object Reference"))
  (returns (Continue :type Boolean))
  (if (`self.Active`)
    (cast `/Game/EmptiveEscort/Escort/BP_EscortBase` Actor
      (:`then`
        (return true))
      (:`CastFailed`
        _)))
  (return false))

(fn `SetActive`
  (params (Active :type Boolean) (Announce :type Boolean))
  (bind _output_get (set `self.Active` Active))
  (if _output_get
    (`PaperSpriteComponent.SetSprite` (`self.WaypointSprite`) (`self.ActiveSprite`))
    (else
      (`PaperSpriteComponent.SetSprite` (`self.WaypointSprite`) (`self.DisabledSprite`))
      (`SceneComponent.SetVisibility` (`self.TextRender`) false false)
      (`SceneComponent.SetVisibility` (`self.TimerFlipbook`) false false)))
  (`SceneComponent.SetVisibility` (`self.EffectFlipbook`) Active false)
  (if Announce
    (message `/Game/EmptiveEscort/Waypoints/BPI_WaypointReceiver.Ping Waypoint Status` (`self.Radio`) self Active))
  (bind _pointofinterest (`self.PointOfInterest`)
    (:`then`
      (`/Game/EmptiveEscort/UserInterface/Minimap/WBP_PointOfInterest.Event Visibility` _pointofinterest Active))
    (:`else`)))

(fn `ShowInProgress`
  (params (`TextVisible?` :type Boolean) (`TimerVisible?` :type Boolean))
  (bind _textrender (`self.TextRender`))
  (bind _timerflipbook (`self.TimerFlipbook`))
  (`SceneComponent.SetVisibility` _textrender `TextVisible?` false)
  (`TextRenderComponent.K2_SetText` _textrender (`self.InProgressText`))
  (if `TimerVisible?`
    (`PaperFlipbookComponent.SetPlaybackPosition` _timerflipbook 0.0 false)
    (`SceneComponent.SetVisibility` _timerflipbook true false)
    (`PaperFlipbookComponent.SetPlayRate` _timerflipbook (/ 1.0 (`self.TimerDuration`)))))

(fn `UserConstructionScript`
  (bind _waypointsprite (`self.WaypointSprite`))
  (bind (_returnvalue_roll _returnvalue_pitch) (`KismetMathLibrary.BreakRotator` (`SceneComponent.K2_GetComponentRotation` _waypointsprite)))
  (`SceneComponent.K2_SetWorldRotation` _waypointsprite (`KismetMathLibrary.MakeRotator` _returnvalue_roll _returnvalue_pitch (`KismetMathLibrary.RandomFloatInRange` -180.0 180.0)) false false))