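; BP_Wall01_Gate is a wall gate that opens during the Mission phase and closes during Rest.
; The PingPhase event calls ToggleOpen, which sets the open state and disables Box collision when open or restores it when closed.
; UpdateSprite then swaps the EW and NS sprite variants to match and hands off to the parent's sprite update.
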(event `/Game/EmptiveEscort/Waypoints/BPI_WaypointReceiver.Ping Phase`
  (params (Phase :type "/Game/EmptiveEscort/Waypoints/EPhase Enum" :default "NewEnumerator0"))
  (switch `/Game/EmptiveEscort/Waypoints/EPhase` Phase
    (:`NewEnumerator0`
      (`self.ToggleOpen` false))
    (:`NewEnumerator1`
      (`self.ToggleOpen` true))))

(fn `ToggleOpen`
  (params (Open :type Boolean))
  (bind _box (`self.Box`))
  (if Open
    (set `self.Open` true)
    (`PrimitiveComponent.SetCollisionEnabled` _box "NoCollision")
    (else
      (set `self.Open` false)
      (`PrimitiveComponent.SetCollisionEnabled` _box "QueryAndPhysics")))
  (`self.UpdateSprite`))

(fn `UpdateSprite`
  (if (`self.Open`)
    (set `self.EW` (`self.EW_Open`))
    (set `self.NS` (`self.NS_Open`))
    (else
      (set `self.NS` (`self.NS_Closed`))
      (set `self.EW` (`self.EW_Closed`))))
  (`parent.UpdateSprite`))

(fn `UserConstructionScript`
  (`parent.UserConstructionScript`))