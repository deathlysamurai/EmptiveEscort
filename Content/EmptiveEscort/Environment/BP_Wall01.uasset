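; Wall environment Blueprint that matches its Paper2D sprite to the direction the wall faces.
; The construction script calls UpdateSprite, which reads the sprite component's world yaw.
; Yaw within the 90-degree bands centered on 90 or 270 selects the NS sprite, and any other yaw selects EW.
; The event graph has no runtime logic.
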(event `self.ReceiveBeginPlay`)

(fn `UpdateSprite`
  (bind _papersprite (`self.PaperSprite`))
  (bind (_returnvalue_roll _returnvalue_pitch _returnvalue_yaw) (`KismetMathLibrary.BreakRotator` (`SceneComponent.K2_GetComponentRotation` _papersprite)))
  (if (or (and (>= _returnvalue_yaw 45.0) (<= _returnvalue_yaw 135.0)) (and (>= _returnvalue_yaw 225.0) (<= _returnvalue_yaw 315.0)))
    (`PaperSpriteComponent.SetSprite` _papersprite (`self.NS`))
    (else
      (`PaperSpriteComponent.SetSprite` _papersprite (`self.EW`)))))

(fn `UserConstructionScript`
  (`self.UpdateSprite`))