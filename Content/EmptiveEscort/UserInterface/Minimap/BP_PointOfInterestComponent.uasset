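; Actor component that marks its owner as a point of interest on the player's minimap.
; On BeginPlay it asks the minimap widget in the player HUD's info overlay to add a POI for the owner and stores the result.
; On EndPlay it removes that minimap marker.
; Equivalent logic for a large map widget, found by class lookup, is present but disconnected.
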(event `self.ReceiveBeginPlay`
  (bind _asplayer_hud (cast `/Game/EmptiveEscort/UserInterface/HUD/PlayerHUD` (`PlayerController.GetHUD` (`GameplayStatics.GetPlayerController` 0))))
  (bind _hudreference (`/Game/EmptiveEscort/UserInterface/HUD/PlayerHUD.HUDReference` _asplayer_hud)
    (:`then`
      (bind _poiwidget (`/Game/EmptiveEscort/UserInterface/Minimap/WBP_Minimap.AddPOI` (`/Game/EmptiveEscort/UserInterface/HUD/PlayerInfo.WBP_Minimap` (`/Game/EmptiveEscort/UserInterface/HUD/HUDCanvas.PlayerInfoOverlay` _hudreference)) (`self.GetOwner`))) ; Adds to minimap
      (set `self.MiniPOI` _poiwidget))
    (:`else`)))

(event `self.ReceiveEndPlay`
  (params (EndPlayReason :type "EEndPlayReason Enum" :default "Destroyed"))
  (bind _minipoi (`self.MiniPOI`)
    (:`then`
      (`Widget.RemoveFromParent` _minipoi))
    (:`else`)))