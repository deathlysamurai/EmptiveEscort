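; BP_EscortBase is the base escort character, which walks toward the nearest waypoint in its active set.
; Initialize seeds the waypoint array, and UpdateWaypointStatus adds or removes a waypoint as it is activated or deactivated.
; Both then call MoveToWaypoint, which uses Simple Move To Actor on the closest waypoint or stops movement immediately when none remain.
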(event `/Game/EmptiveEscort/Waypoints/BPI_WaypointReceiver.Update Waypoint Status`
  (params (Waypoint :type "/Game/EmptiveEscort/Waypoints/BP_Waypoint Object Reference") (Active :type Boolean))
  (bind _waypointarray (`self.WaypointArray`))
  (if Active
    (`KismetArrayLibrary.Array_AddUnique` _waypointarray Waypoint)
    (else
      (`KismetArrayLibrary.Array_RemoveItem` _waypointarray Waypoint)))
  (`self.Move To Waypoint` _waypointarray))

(event `self.ReceiveBeginPlay`)

(fn `Initialize`
  (params (Waypoints :type "Array of /Game/EmptiveEscort/Waypoints/BP_Waypoint Object Reference"))
  (bind _output_get (set `self.WaypointArray` Waypoints))
  (`self.Move To Waypoint` _output_get))

(fn `Move To Waypoint`
  (params (Waypoints :type "Array of /Game/EmptiveEscort/Waypoints/BP_Waypoint Object Reference"))
  (if (> (`KismetArrayLibrary.Array_Length` Waypoints) 0)
    (`AIBlueprintHelperLibrary.SimpleMoveToActor` (`self.GetController`) (`.ReturnValue` (`GameplayStatics.FindNearestActor` (`self.K2_GetActorLocation`) Waypoints)))
    (else
      (`MovementComponent.StopMovementImmediately` (`self.CharacterMovement`)))))

(fn `UserConstructionScript`)