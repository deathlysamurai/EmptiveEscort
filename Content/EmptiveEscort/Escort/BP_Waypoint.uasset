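; BP_Waypoint is a waypoint actor for the escort that tracks whether it is still active.
; On BeginPlay it shows its active material, finds BP_Escort in the level and registers itself as active through UpdateWaypoints.
; When that escort overlaps it while active, it switches to the disabled material, turns inactive and notifies the escort through the same call.
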(event `self.ReceiveBeginPlay`
  (`PrimitiveComponent.SetMaterial` (`self.Cylinder`) 0 (`self.ActiveMaterial`))
  (bind _returnvalue (`GameplayStatics.GetActorOfClass` "/Game/EmptiveEscort/Escort/BP_Escort.BP_Escort_C"))
  (bind _output_get (set `self.Escort` _returnvalue))
  (`/Game/EmptiveEscort/Escort/BP_Escort.Update Waypoints` _output_get self true))

(event `self.ReceiveActorBeginOverlap`
  (params (OtherActor :type "Actor Object Reference"))
  (if (and (== OtherActor (`self.Escort`)) (`self.Active`))
    (`PrimitiveComponent.SetMaterial` (`self.Cylinder`) 0 (`self.DisabledMaterial`))
    (set `self.Active` false)
    (`/Game/EmptiveEscort/Escort/BP_Escort.Update Waypoints` (`self.Escort`) self false)))

(fn `UserConstructionScript`)