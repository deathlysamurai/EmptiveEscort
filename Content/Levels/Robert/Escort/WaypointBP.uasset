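; WaypointBP is an actor in the Escort level folder that acts as a one-shot waypoint marker.
; It shows an active material on its Cylinder when play begins.
; When an actor carrying the target tag overlaps it while active, it switches to a disabled material and clears its Active flag, with no path to reactivate it within this Blueprint.
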(event `self.ReceiveBeginPlay`
  (`PrimitiveComponent.SetMaterial` (`self.Cylinder`) 0 (`self.ActiveMaterial`)))

(event `self.ReceiveActorBeginOverlap`
  (params (OtherActor :type "Actor Object Reference"))
  (if (and (`self.ActorHasTag` OtherActor (`self.TargetTag`)) (`self.Active`))
    (`PrimitiveComponent.SetMaterial` (`self.Cylinder`) 0 (`self.DisabledMaterial`))
    (set `self.Active` false)))

(fn `UserConstructionScript`)