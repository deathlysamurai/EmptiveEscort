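; Escort character that walks toward the nearest active waypoint in the level.
; UpdateWaypoints adds or removes a waypoint from its array, then sends its controller to the closest remaining one with SimpleMoveToActor.
; Movement stops immediately when the array is empty.
; The target is re-evaluated only when that event fires, as there is no Tick logic.
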(event `/Game/Levels/Robert/Escort/BPI_Waypoint.Update Waypoints`
  (params (Waypoint :type "/Game/Levels/Robert/Escort/BP_Waypoint Object Reference") (Active :type Boolean))
  (bind _waypointarray (`self.WaypointArray`))
  (bind _waypointarray_2 (`self.WaypointArray`))
  (if Active
    (`KismetArrayLibrary.Array_AddUnique` _waypointarray Waypoint)
    (else
      (`KismetArrayLibrary.Array_RemoveItem` _waypointarray Waypoint)))
  (if (> (`KismetArrayLibrary.Array_Length` _waypointarray_2) 0)
    (`AIBlueprintHelperLibrary.SimpleMoveToActor` (`self.GetController`) (`.ReturnValue` (`GameplayStatics.FindNearestActor` (`self.K2_GetActorLocation`) _waypointarray_2)))
    (else
      (`MovementComponent.StopMovementImmediately` (`self.CharacterMovement`)))))

(event `self.ReceiveBeginPlay`)

(fn `UserConstructionScript`)